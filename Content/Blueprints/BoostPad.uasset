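; BoostPad is a trigger actor that launches the player character when they overlap its box.
; It zeroes the character's velocity, air control and ground friction, first saving air control into the character's BaseAirControl; nothing here restores them.
; The launch uses configurable X and Z speeds, scaling X by the pad's forward X component and leaving Y unset.
; A DoOnce gate re-arms the pad after a short delay.
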(event `self.Box.OnComponentBeginOverlap`
  (params (OverlappedComponent :type "PrimitiveComponent Object Reference") (OtherActor :type "Actor Object Reference") (OtherComp :type "PrimitiveComponent Object Reference") (OtherBodyIndex :type Integer) (bFromSweep :type Boolean) (SweepResult :type "HitResult Structure (by ref)"))
  (bind _returnvalue_x (`KismetMathLibrary.BreakVector` (`KismetMathLibrary.GetForwardVector` (`self.K2_GetActorRotation`))))
  (bind _asbp_player_character (cast `/Game/Character/Player/BP_PlayerCharacter` OtherActor))
  (`/Engine/EditorBlueprintResources/StandardMacros.DoOnce` false :!label _label
    (:`Completed`
      (bind _charactermovement (`Character.CharacterMovement` _asbp_player_character))
      (set `MovementComponent.Velocity` (0.0 0.0 0.0) _charactermovement)
      (set `/Game/Character/Player/BP_PlayerCharacter.Base_Air_Control` (`CharacterMovementComponent.AirControl` _charactermovement) _asbp_player_character)
      (set `CharacterMovementComponent.AirControl` 0.0 _charactermovement)
      (set `CharacterMovementComponent.GroundFriction` 0.0 _charactermovement)
      (`|ExecutionSequence`
        (:`then_0`
          (`Character.LaunchCharacter` _asbp_player_character (`KismetMathLibrary.MakeVector` (* _returnvalue_x (`self.X_Velocity`)) 0.0 (`self.Z_Velocity`)) false true))
        (:`then_1`
          (`KismetSystemLibrary.Delay` 2.0)
          (goto _label :!via `Reset`))))))

(fn `UserConstructionScript`)