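; PU_Parent is a power-up pickup, apparently a base for variants, that grants a Gameplay Ability System effect to the player.
; A timeline on BeginPlay drives the cube's height and yaw to make it hover and spin.
; When a BP_PlayerCharacter overlaps the box, the configured Effect is applied to its ability system component and the pickup destroys itself.
; BeginPlay also prints a label for speed or jump effects, matched by class display name.
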(event `self.ReceiveBeginPlay`
  (bind _cube (`self.Cube`))
  (bind (_relativelocation_x _relativelocation_y) (`KismetMathLibrary.BreakVector` (`SceneComponent.RelativeLocation` _cube)))
  (`|ExecutionSequence`
    (:`then_0`
      ;[1 1 1] Hovering Timeline
      (bind (_direction _hovering _rotating) (`Timeline|Hovering`)
        (:`Update`
          (`SceneComponent.K2_SetRelativeLocationAndRotation` _cube (`KismetMathLibrary.MakeVector` _relativelocation_x _relativelocation_y _hovering) (`KismetMathLibrary.MakeRotator` 0.0 0.0 (* _rotating 100.0)) false false))))
    (:`then_1`
      (switch `string` (`KismetSystemLibrary.GetClassDisplayName` (`self.Effect`))
        (:`GE_Speed_C`
          (`KismetSystemLibrary.PrintString` "SPEED"))
        (:`GE_Jump_C`
          (`KismetSystemLibrary.PrintString` "JUMP"))))))

(event `self.Box.OnComponentBeginOverlap`
  (params (OverlappedComponent :type "PrimitiveComponent Object Reference") (OtherActor :type "Actor Object Reference") (OtherComp :type "PrimitiveComponent Object Reference") (OtherBodyIndex :type Integer) (bFromSweep :type Boolean) (SweepResult :type "HitResult Structure (by ref)"))
  (bind _asbp_player_character (cast `/Game/Character/Player/BP_PlayerCharacter` OtherActor))
  (`AbilitySystemComponent.BP_ApplyGameplayEffectToSelf` :`self` (`AbilitySystemBlueprintLibrary.GetAbilitySystemComponent` _asbp_player_character) :`GameplayEffectClass` (`self.Effect`) :`Level` 0.0)
  (`self.K2_DestroyActor`))

(fn `UserConstructionScript`)