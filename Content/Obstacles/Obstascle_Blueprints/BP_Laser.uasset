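; Laser obstacle with a scalable beam and death zone that can move, swing, spin or blink, per its flags.
; BeginPlay sizes the beam and starts the enabled behaviors, with swinging disabling spin.
; Self-restarting timelines lerp the laser, using counter parity to reverse movement and swing each pass.
; Alternating loops on delays, hiding the beam and switching off the DeathZone_Laser found by matching the actor's location.
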(event `self.ReceiveBeginPlay`
  ;[1 1 1] Sets Laser Length
  (`SceneComponent.SetRelativeScale3D` (`self.DeathZone_Laser`) (`KismetMathLibrary.MakeVector` 0.1 (* (`self.Laser Length`) (`self.BeamLength`)) 0.05))
  (`SceneComponent.SetRelativeScale3D` (`self.SM_Laser_beam`) (`KismetMathLibrary.MakeVector` 0.2 0.2 (`self.Laser Length`)))
  (if (`self.Move`)
    (`self.LaserMove`)
    (`TimelineComponent.SetPlayRate` (`self.Movement_Timeline`) (`self.MoveSpeed`)))
  ;[1 1 1] If Swinging & Spinning are True, Set Spinning False
  (if (`self.Rotate`)
    (`self.LaserSwinging`)
    (`TimelineComponent.SetPlayRate` (`self.Rotate_Timeline`) (`self.Rotate Speed`))
    (bind _output_get (set `self.Spin` false)))
  (if _output_get
    (`self.Spinning`)
    (`TimelineComponent.SetPlayRate` (`self.Spinning Timeline`) (`self.SpinSpeed`)))
  (if (`self.Alternate`)
    (`self.Alternating`)))

(event `LaserSwinging`
  ;[1 1 1] Rotate
  (`self.Las_Rotate`)
  (bind (_direction _newtrack_0) (`Timeline|Rotate_Timeline` :!via `PlayFromStart`)
    (:`Update`
      (`SceneComponent.K2_SetRelativeRotation` (`self.laserthing`) (`KismetMathLibrary.RLerp` (`self.Las_Start_Val`) (`self.Las_End_Val`) _newtrack_0) false false))
    (:`Finished`
      (`self.LaserSwinging`))))

(event `LaserMove`
  ;[1 1 1] Moving
  (`self.Las_Move`)
  (bind (_direction _newtrack_0) (`Timeline|Movement_Timeline` :!via `PlayFromStart`)
    (:`Update`
      (`SceneComponent.K2_SetRelativeTransform` (`self.laserthing`) (`KismetMathLibrary.TLerp` (`KismetMathLibrary.Conv_VectorToTransform` (`self.Las_Loop_Start`)) (`KismetMathLibrary.Conv_VectorToTransform` (`self.Las_Loop_End`)) _newtrack_0) false false))
    (:`Finished`
      (`self.LaserMove`))))

(event `Spinning`
  ;[1 1 1] Spin
  (bind (_direction _spinning) (`Timeline|Spinning Timeline` :!via `PlayFromStart`)
    (:`Update`
      (`SceneComponent.K2_SetRelativeRotation` (`self.laserthing`) (`KismetMathLibrary.RLerp` (`self.Spin_Start`) (`self.Spin_End`) _spinning) false false))
    (:`Finished`
      (`self.Spinning`))))

(event `Alternating`
  ;[1 1 1] Alternating
  (`KismetSystemLibrary.Delay` (`self.Alternating_Interval_On`))
  (`SceneComponent.SetVisibility` (`self.SM_Laser_beam`) false false)
  (bind _outactors (`GameplayStatics.GetAllActorsOfClass` "/Game/Obstacles/Obstascle_Blueprints/DeathZone_Laser.DeathZone_Laser_C"))
  (for _array_element _outactors
    (if (== (`self.K2_GetActorLocation` _array_element) (`self.K2_GetActorLocation`))
      (set `/Game/Obstacles/Obstascle_Blueprints/DeathZone_Laser.On` false _array_element)
      (`KismetSystemLibrary.Delay` (`self.Alternating Interval Off`))
      (set `/Game/Obstacles/Obstascle_Blueprints/DeathZone_Laser.On` true _array_element)
      (`SceneComponent.SetVisibility` (`self.SM_Laser_beam`) true true)
      (`self.Alternating`))))

(fn `Las_Move`
  (set `self.MoveCounter` (+ (`self.MoveCounter`) 1.0))
  (`/Engine/EditorBlueprintResources/StandardMacros.CompareFloat` (mod (`self.MoveCounter`) 2.0)
    (:`>`
      (bind _output_get (set `self.MoveCounterEven` true)))
    (:`==`
      (set `self.MoveCounterEven` false)))
  (if _output_get
    (set `self.Las_Loop_Start` (`self.Las_Start_Pos`))
    (set `self.Las_End_Pos` (`KismetMathLibrary.MakeVector` (`self.MoveDistance`)))
    (set `self.Las_Loop_End` (`self.Las_End_Pos`))
    (else
      (set `self.Las_Loop_Start` (`self.Las_End_Pos`))
      (set `self.Las_Loop_End` (`self.Las_Start_Pos`)))))

(fn `Las_Rotate`
  (set `self.RotateCounter` (+ (`self.RotateCounter`) 1.0))
  (`/Engine/EditorBlueprintResources/StandardMacros.CompareFloat` (mod (`self.RotateCounter`) 2.0)
    (:`>`
      (bind _output_get (set `self.RotateCounterEven` false)))
    (:`==`
      (set `self.RotateCounterEven` true)))
  (if _output_get
    (set `self.Las_Start_Val` (`self.Las_Start_Rot`))
    (set `self.Las_End_Val` (`self.Las_End_Rot`))
    (else
      (set `self.Las_Start_Val` (`self.Las_End_Rot`))
      (set `self.Las_End_Val` (`self.Las_Start_Rot`)))))

(fn `UserConstructionScript`)