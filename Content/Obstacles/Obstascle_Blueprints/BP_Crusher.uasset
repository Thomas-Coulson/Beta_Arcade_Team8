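; Crusher obstacle whose plate repeatedly moves down and back up in an endless loop.
; BeginPlay waits StartOffset before the first Crush, allowing a delayed start per crusher.
; Two timelines, CrusherDown and CrusherUp, chain to lerp the plate's relative transform between CrusherUpLoc and CrusherDownLoc, then call Crush again.
; The plate moves without sweep, and the Blueprint's graphs contain no damage or hit logic.
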(event `self.ReceiveBeginPlay`
  (`KismetSystemLibrary.Delay` (`self.Start Offset`))
  (`self.Crush`))

(event `Crush`
  (bind (_direction _newtrack_0) (`Timeline|Crusher Down` :!via `PlayFromStart`)
    (:`Update`
      (`SceneComponent.K2_SetRelativeTransform` (`self.SM_CrusherPlate`) (`KismetMathLibrary.TLerp` (`KismetMathLibrary.Conv_VectorToTransform` (`self.Crusher Up Loc`)) (`KismetMathLibrary.Conv_VectorToTransform` (`self.Crusher Down Loc`)) _newtrack_0) false false))
    (:`Finished`
      (bind (_direction_2 _newtrack_0_2) (`Timeline|Crusher Up` :!via `PlayFromStart`)
        (:`Update`
          (`SceneComponent.K2_SetRelativeTransform` (`self.SM_CrusherPlate`) (`KismetMathLibrary.TLerp` (`KismetMathLibrary.Conv_VectorToTransform` (`self.Crusher Down Loc`)) (`KismetMathLibrary.Conv_VectorToTransform` (`self.Crusher Up Loc`)) _newtrack_0_2) false false))
        (:`Finished`
          (`self.Crush`))))))

(fn `UserConstructionScript`)