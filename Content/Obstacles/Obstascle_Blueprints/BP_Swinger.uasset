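; BP_Swinger is an obstacle that swings its static mesh back and forth endlessly between two rotations.
; BeginPlay sets the Swinging timeline's play rate from SwingSpeed, then calls Swing.
; Each Swing increments a counter and uses its parity to choose which of RotatorStartVal and RotatorEndVal is the target.
; The timeline lerps the mesh's relative rotation and calls Swing again on finish, forming the loop.
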(event `self.ReceiveBeginPlay`
  (`TimelineComponent.SetPlayRate` (`self.Swinging`) (`self.SwingSpeed`))
  (`self.Swing`))

(event `Swing`
  (set `self.Counter` (+ (`self.Counter`) 1.0))
  (`/Engine/EditorBlueprintResources/StandardMacros.CompareFloat` (mod (`self.Counter`) 2.0)
    (:`>`
      (bind _output_get (set `self.CounterEven` false)))
    (:`==`
      (set `self.CounterEven` true)))
  (if _output_get
    (set `self.StartRotation` (`self.RotatorStartVal`))
    (set `self.TargetRotation` (`self.RotatorEndVal`))
    (bind (_direction _swinging) (`Timeline|Swinging` :!via `PlayFromStart` :!label _label)
      (:`Update`
        (`SceneComponent.K2_SetRelativeRotation` (`self.StaticMesh`) (`KismetMathLibrary.RLerp` (`self.StartRotation`) (`self.TargetRotation`) _swinging) false false))
      (:`Finished`
        (`self.Swing`)))
    (else
      (set `self.StartRotation` (`self.RotatorEndVal`))
      (set `self.TargetRotation` (`self.RotatorStartVal`))
      (goto _label :!via `PlayFromStart`))))

(fn `UserConstructionScript`)