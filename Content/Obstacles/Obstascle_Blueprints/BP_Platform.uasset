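; BP_Platform is an obstacle platform that slides back and forth endlessly between a start location and a point set by Distance along negative relative Y.
; BeginPlay sets the Movement timeline's play rate from MoveSpeed and calls Move.
; Move uses counter parity to swap the endpoints, then replays the timeline to lerp SMPlatform's relative transform without sweeping.
; Each finished timeline calls Move again.
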(event `self.ReceiveBeginPlay`
  (`TimelineComponent.SetPlayRate` (`self.Movement`) (`self.MoveSpeed`))
  (`self.Move`))

(event `Move`
  (set `self.Counter` (+ (`self.Counter`) 1.0))
  (`/Engine/EditorBlueprintResources/StandardMacros.CompareFloat` (mod (`self.Counter`) 2.0)
    (:`>`
      (bind _output_get (set `self.CounterEven` true)))
    (:`==`
      (set `self.CounterEven` false)))
  (if _output_get
    (set `self.LoopStart` (`self.LocStart`))
    (set `self.LocEnd` (`KismetMathLibrary.MakeVector` 0.0 (- 0.0 (`self.Distance`))))
    (set `self.LoopEnd` (`self.LocEnd`))
    (bind (_direction _movement) (`Timeline|Movement` :!via `PlayFromStart` :!label _label)
      (:`Update`
        (`SceneComponent.K2_SetRelativeTransform` (`self.SM_Platform`) (`KismetMathLibrary.TLerp` (`KismetMathLibrary.Conv_VectorToTransform` (`self.LoopStart`)) (`KismetMathLibrary.Conv_VectorToTransform` (`self.LoopEnd`)) _movement) false false))
      (:`Finished`
        (`self.Move`)))
    (else
      (set `self.LoopStart` (`self.LocEnd`))
      (set `self.LoopEnd` (`self.LocStart`))
      (goto _label :!via `PlayFromStart`))))

(fn `UserConstructionScript`)