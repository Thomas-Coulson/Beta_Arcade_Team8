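; BP_GameMode is a game mode that stores the player's spawn location and handles the win event, ChickenDinner.
; InitSpawn saves the given location to PlayerSpawn.
; ChickenDinner pauses a timer and prints its current time in seconds.
; An unconnected draft for an end screen creates a widget without a set class, switches input to UI only and shows the cursor, but never runs.
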(event `self.ReceiveBeginPlay`)

(event `Init Spawn`
  (params (SpawnLocation :type "Vector Structure"))
  (set `self.PlayerSpawn` SpawnLocation))

(event `Chicken Dinner`
  (`|ExecutionSequence`
    (:`then_1`
      (`self.PauseTimer` true)
      (bind _returnvalue (`self.GetCurrentTimeSecconds`))
      (`KismetSystemLibrary.PrintString` (`KismetStringLibrary.Conv_DoubleToString` _returnvalue)))))

(fn `UserConstructionScript`)